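; Base zombie character Blueprint with an Fsm component that exposes health, state, damage and activate/deactivate actions.
; Its graph has almost no live logic: BeginPlay and Tick are empty, and actor overlap only casts to BP_ClimbOverZone.
; The rest is disconnected debug and test code for FSM state, climb-over, avoidance, ragdoll reset and pooling-style reactivation, including the binding for the placeholder hit handler.
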(event Custom|OnActorHit_Event
  (params (SelfActor :type Actor%20Object%20Reference) (OtherActor :type Actor%20Object%20Reference) (NormalImpulse :type Vector) (Hit :type Hit%20Result%20Structure%20%28by%20ref%29))
  (Development|PrintString "Hello"))

(event EventBeginPlay)

(event EventTick
  (params (DeltaSeconds :type Float%20%28single-precision%29)))

(event Collision|EventActorBeginOverlap
  (params (OtherActor :type Actor%20Object%20Reference))
  (Utilities|Casting|CastToBP_ClimbOverZone OtherActor))

(fn ConstructionScript)