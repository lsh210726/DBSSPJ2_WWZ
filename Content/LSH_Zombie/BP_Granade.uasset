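; BP_Granade is a grenade actor that explodes when it hits something, damaging and launching nearby zombies.
; On Hit, a sphere trace on the Visibility channel finds BP_LSH_BaseZom actors around the impact and calls their FSM damage process.
; Each zombie's ragdoll bodies get an outward, upward-biased impulse with clamped inverse-square distance falloff.
; It then spawns a Niagara explosion and destroys itself.
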(event Collision|EventHit
  (params (MyComp :type Primitive%20Component%20Object%20Reference) (Other :type Actor%20Object%20Reference) (OtherComp :type Primitive%20Component%20Object%20Reference) (bSelfMoved :type Boolean) (HitLocation :type Vector :default "0, 0, 0") (HitNormal :type Vector :default "0, 0, 0") (NormalImpulse :type Vector :default "0, 0, 0") (Hit :type Hit%20Result%20Structure%20%28by%20ref%29))
  (bind _returnvalue (Transformation|GetActorLocation))
  (bind _returnvalue_2 (Math|Float|MakeLiteralFloat 1e+07))
  (bind _outhits (Collision|MultiSphereTraceByChannel HitLocation HitLocation 2.5e+02 "TraceTypeQuery1" false 0 "None"))
  (for _array_element _outhits
    (bind _asbp_lsh_base_zom (Utilities|Casting|CastToBP_LSH_BaseZom (.HitActor (Collision|BreakHitResult _array_element))))
    (Class|LSHEnemyFSM|OnDamageProcess (Variables|/Script/WWZ.LSH_BaseZom|Getfsm _asbp_lsh_base_zom) 4)
    (Class|SkeletalMeshComponent|AddImpulsetoAllBodiesBelow (Variables|/Script/Engine.Character|GetMesh _asbp_lsh_base_zom) (* (Math|Vector|Normalize (+ (- (Transformation|GetActorLocation _asbp_lsh_base_zom) _returnvalue) "0.000000,0.000000,200.000000")) (Math|Float|Clamp(Float) (/ _returnvalue_2 (Math|Float|Power (Math|Vector|Distance(Vector) _returnvalue (Transformation|GetActorLocation _asbp_lsh_base_zom)) 2.0)) 3e+03 _returnvalue_2)) "None" false true))
  (Niagara|SpawnSystematLocation "/Game/Realistic_Starter_VFX_Pack_Niagara/Niagara/Explosion/NS_Explosion_Grenade.NS_Explosion_Grenade" (Transformation|GetActorLocation))
  (Actor|DestroyActor))

(event Collision|EventActorBeginOverlap
  (params (OtherActor :type Actor%20Object%20Reference)))

(event EventTick
  (params (DeltaSeconds :type Float%20%28single-precision%29)))

(event EventBeginPlay)

(fn ConstructionScript)