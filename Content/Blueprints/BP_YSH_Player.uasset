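; Player Blueprint that creates a crosshair widget (WBP_Crosshair) on BeginPlay.
; That creation is its only live logic, and the widget is not added to the viewport on that path.
; Disconnected fragments remain for a timed crosshair flag, a reload widget, an animation start and delayed visibility toggles, none of which run.
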(event EventBeginPlay
  (UserInterface|CreateWidget "/Game/UI/WBP_Crosshair.WBP_Crosshair_C"))

(event Collision|EventActorBeginOverlap
  (params (OtherActor :type Actor%20Object%20Reference)))

(event EventTick
  (params (DeltaSeconds :type Float%20%28single-precision%29)))

(event Input|ActionEvents|InputActionFire
  (params (Key :type Key%20Structure)))

(fn ConstructionScript)