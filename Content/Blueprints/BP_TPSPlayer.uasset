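; BP_TPSPlayer is a third-person shooter player Blueprint whose only active logic is hitscan firing.
; Pressing Fire runs a Visibility line trace from the camera along its forward vector, with debug drawing.
; A hit on a physics-simulating component receives a mass-scaled force along the trace direction.
; Movement, look, jump, lerped FOV zoom and projectile spawning exist only as disconnected nodes that never run.
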(event EventBeginPlay)

(event Collision|EventActorBeginOverlap
  (params (OtherActor :type Actor%20Object%20Reference)))

(event EventTick
  (params (DeltaSeconds :type Float%20%28single-precision%29))
  ;[1 1 1] 스무스하게 Zoom In/Out 하기(Lerp함수 사용)
)

(event Input|ActionEvents|InputActionJump
  (params (Key :type Key%20Structure)))

(event Input|ActionEvents|InputActionFire
  (params (Key :type Key%20Structure))
  (bind _cameracomp (Variables|Default|GetcameraComp))
  (bind _returnvalue (Transformation|GetWorldLocation _cameracomp))
  ;[1 1 1] BP_총발사
  ;;[1 1 1] Linetrace로 총쏘기(총이 나가는구간에 충돌이있는가)
  (:Pressed
    (bind (_outhit _returnvalue_2) (Collision|LineTraceByChannel _returnvalue (+ _returnvalue (* (Math|Vector|GetForwardVector _cameracomp) 1e+05)) "TraceTypeQuery1" false 0 "ForDuration"))
    (if _returnvalue_2
      (if (Physics|IsSimulatingPhysics (.HitComponent (Collision|BreakHitResult _outhit)) "None")
        (Physics|AddForce (.HitComponent (Collision|BreakHitResult _outhit)) (* (Math|Vector|Normalize (- (.TraceEnd (Collision|BreakHitResult _outhit)) (.TraceStart (Collision|BreakHitResult _outhit)))) 5e+05 (Physics|GetMass (.HitComponent (Collision|BreakHitResult _outhit)))) "None" false)))))

(event Input|ActionEvents|InputActionZoom
  (params (Key :type Key%20Structure))
  ;[1 1 1] 스무스하게 Zoom In/Out 하기(Lerp함수 사용)
  ;;[1 1 1] Zoom으로 Widget왔다갔다하기(클릭)-기본
)

(event Input|AxisEvents|InputAxisLookUp/DownMouse
  (params (AxisValue :type Float%20%28single-precision%29)))

(event Input|AxisEvents|InputAxisTurnRight/LeftMouse
  (params (AxisValue :type Float%20%28single-precision%29)))

(fn ConstructionScript)